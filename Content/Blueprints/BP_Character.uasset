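; BP_Character is a player character that moves where its camera looks and detects red and blue cubes by gaze.
; Holding touch sets the speed, and Tick applies movement input along the camera's forward vector, scaled by delta time.
; Each Tick, GazeCheck also runs a debug-drawn line trace from the camera and prints a colored message when it hits a BP_RedCube or BP_BlueCube.
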(event `self.ReceiveTick`
  (params (DeltaSeconds :type "Float (single-precision)"))
  (`self.GazeCheck`)
  (`self.AddMovementInput` (`KismetMathLibrary.GetForwardVector` (`SceneComponent.K2_GetComponentRotation` (`self.Camera`))) (* (`self.CurrentSpeed`) (`GameplayStatics.GetWorldDeltaSeconds`))))

(event `InputAction|Touch`
  (params (Key :type "Key Structure"))
  (:`Pressed`
    (set `self.CurrentSpeed` (`self.Move Speed`)))
  (:`Released`
    (set `self.CurrentSpeed` 0.0)))

(event `GazeCheck`
  (bind _camera (`self.Camera`))
  (bind _returnvalue (`SceneComponent.K2_GetComponentLocation` _camera))
  ;[1 1 1] GazeCheck
  (bind _outhit (`KismetSystemLibrary.LineTraceSingle` :`Start` _returnvalue :`End` (+ (* (`SceneComponent.GetForwardVector` _camera) 2000.0) _returnvalue) :`TraceChannel` "TraceTypeQuery1" :`DrawDebugType` "ForOneFrame" :`TraceColor` (struct :`R` 0.911209 :`G` 1.0 :`B` 0.900152 :`A` 1.0)))
  (bind (_bblockinghit _binitialoverlap _time _distance _location _impactpoint _normal _impactnormal _physmat _hitactor) (`GameplayStatics.BreakHitResult` _outhit))
  (cast `/Game/Blueprints/BP_RedCube` _hitactor
    (:`then`
      (`KismetSystemLibrary.PrintString` "Red Cube Found" true true (struct :`R` 0.433333 :`B` 0.102139 :`A` 1.0)))
    (:`CastFailed`
      (cast `/Game/Blueprints/BP_BlueCube` _hitactor)
      (`KismetSystemLibrary.PrintString` "Blue Cube Found" true true (struct :`R` 0.04925 :`G` 0.02838 :`B` 0.433333 :`A` 1.0)))))

(fn `UserConstructionScript`)